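; Melee enemy NPC that starts as a lying body and, on WakeUp, swaps it for the visible character mesh and health bar.
; Punch uses timed delays to damage the player pawn without a range check, then randomizes the next attack side.
; Damage updates a widget health bar turned by player yaw; death stops movement, then drops a random item and destroys the actor.
; Getters expose lying, attacking and death state; RagdolHim is never called here.
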(event Custom|Die
  (CallFunction|DisableHPBar)
  (Pawn|Components|CharacterMovement|DisableMovement (Variables|Character|GetCharacterMovement))
  (Utilities|FlowControl|Delay 5.0)
  (CallFunction|DropItem)
  (Actor|DestroyActor))

(event Game|Damage|EventAnyDamage
  (params (Damage :type Float%20%28single-precision%29) (DamageType :type Damage%20Type%20Object%20Reference) (InstigatedBy :type Controller%20Object%20Reference) (DamageCauser :type Actor%20Object%20Reference))
  (if (<= (- (Variables|Default|GetCurentHealth) Damage) 0.0)
    (Variables|Default|SetCurentHealth 0.0)
    (CallFunction|Die)
    (else
      (Variables|Default|SetCurentHealth (- (Variables|Default|GetCurentHealth) Damage))
      (CallFunction|UpdateHPBar))))

(event EventBeginPlay
  (CallFunction|UpdateHPBar))

(event EventTick
  (params (DeltaSeconds :type Float%20%28single-precision%29))
  (CallFunction|FrontHPBartoPlayer))

(event EventShotat
  (params (target :type Actor%20Object%20Reference))
  (Variables|Default|SetAttacking true)
  (Utilities|FlowControl|Delay 1.0)
  (Variables|Default|SetAttacking false))

(event EventPunch
  (params (target :type Actor%20Object%20Reference))
  (Variables|Default|SetAttacking true)
  (Utilities|FlowControl|Delay 1.4)
  (Game|Damage|ApplyDamage (Game|Player|GetPlayerPawn 0) 15.0 0 0)
  (Utilities|FlowControl|Delay 1.0)
  (Variables|Default|SetAttacking false)
  (Variables|Default|SetLeftAttack (> (Math|Random|RandomInteger 2) 0)))

(event EventWakeUp
  (params (target :type Actor%20Object%20Reference))
  (Variables|Default|SetLying false)
  (Rendering|SetVisibility (Variables|Default|GetHPBar) true false)
  (Rendering|SetVisibility (Variables|Character|GetMesh) true false)
  (Rendering|SetVisibility (Variables|Default|GetLyingBody) false false))

(fn ConstructionScript)

(fn NewFunction0)

(fn RagdolHim
  (Physics|SetSimulatePhysics (Variables|Character|GetMesh) true)
  (Components|Activation|Deactivate (Variables|Character|GetCharacterMovement))
  (Components|Activation|Deactivate (Variables|Collision|GetCapsuleComponent))
  (Class|Pawn|DetachfromControllerPendingDestroy))

(fn UpdateHPBar
  (bind _asnpc_hp (Utilities|Casting|CastToNPC_HP (UserInterface|GetWidget (Variables|Default|GetHPBar))))
  (Variables|/Game/DiffStuff/AI/UI/NPC_HP.NPC_HP_C|SetHealthPercentage _asnpc_hp (/ (Variables|Default|GetCurentHealth) (Variables|Default|GetMaxHealth)))
  (return))

(fn DisableHPBar
  (bind _asnpc_hp (Utilities|Casting|CastToNPC_HP (UserInterface|GetWidget (Variables|Default|GetHPBar))))
  (Widget|SetVisibility _asnpc_hp "Hidden"))

(fn FrontHPBartoPlayer
  (bind _hpbar (Variables|Default|GetHPBar))
  (bind _returnvalue (Transformation|GetWorldRotation _hpbar))
  (Transformation|SetWorldRotation _hpbar (Math|Rotator|MakeRotator (.roll _returnvalue) (.pitch _returnvalue) (- (.yaw (Transformation|GetActorRotation (Game|Player|GetPlayerPawn 0))) 1.8e+02)) false false))

(fn DropItem
  (bind _dropableitem (Variables|Default|GetDropableItem))
  (Game|SpawnActorfromClass (Utilities|Array|Get(acopy) _dropableitem (Math|Random|RandomInteger (Utilities|Array|Length _dropableitem))) (Math|Conversions|ToTransform(Vector) (Transformation|GetActorLocation self)) "Undefined" 0 0))

(fn IsAttacking
  (return (Variables|Default|GetAttacking)))

(fn IsDead
  (return (<= (Variables|Default|GetCurentHealth) 0.0)))

(fn IsLeftAttack
  (return (Variables|Default|GetLeftAttack)))

(fn IsLying
  (return (Variables|Default|GetLying)))

(fn IsSlinger
  (return false))